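; BP_Dummy is a damageable target character with an overhead-style health bar widget.
; On any damage it launches along the player character's facing direction, plays an axe hit sound at its location and passes the damage to BPCPlayerStats.
; When DecreaseHealth returns true, the health bar is hidden.
; BeginPlay caches the WB_DummyHealth widget, and an unconnected montage node never runs.
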(event Game|Damage|EventAnyDamage
  (params (Damage :type Float%20%28single-precision%29) (DamageType :type Damage%20Type%20Object%20Reference) (InstigatedBy :type Controller%20Object%20Reference) (DamageCauser :type Actor%20Object%20Reference))
  (bind _asbp_third_person_character (Utilities|Casting|CastToBP_ThirdPersonCharacter (Game|GetPlayerCharacter 0)))
  (Character|LaunchCharacter (* (Math|Vector|GetForwardVector (Transformation|GetActorRotation _asbp_third_person_character)) 7e+02) false false)
  (Audio|PlaySoundatLocation "/Game/Audio/Axe_HIts/Axe_Hit_2.Axe_Hit_2" (Transformation|GetActorLocation) "0, 0, 0" 1.0 1.0 0.0 0 0 0 0)
  (bind _is_player_dead_ (Default|DecreaseHealth (Variables|Default|GetBPC_PlayerStats) Damage))
  (if _is_player_dead_
    (Rendering|SetVisibility (Variables|Default|GetHealth%20Bar%20Widget) false false)))

(event EventBeginPlay
  (bind _aswb_dummy_health (Utilities|Casting|CastToWB_DummyHealth (UserInterface|GetWidget (Variables|Default|GetHealth%20Bar%20Widget))))
  (Variables|Default|SetHealthBar%20UI _aswb_dummy_health))

(fn ConstructionScript)